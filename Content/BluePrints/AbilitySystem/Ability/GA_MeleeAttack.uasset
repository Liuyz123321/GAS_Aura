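; Gameplay ability that performs a melee attack for an avatar implementing the combat interface.
; On activation it faces the avatar toward its target actor and plays the attack montage supplied by the avatar.
; The montage's tagged gameplay event triggers a single small-radius sphere query at that tag's weapon socket, damaging live players found other than the avatar.
; The ability ends when the montage completes, is interrupted or is cancelled.
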(event Ability|EventActivateAbility
  (bind _returnvalue (Ability|GetAvatarActorfromActorInfo))
  (bind _returnvalue_2 (Ability|GetAvatarActorfromActorInfo))
  (bind _returnvalue_3 (Ability|GetAvatarActorfromActorInfo))
  (bind _returnvalue_4 (Class|EnemyInterface|GetTargetActor(Message) _returnvalue))
  (bind _ascombat_interface (Utilities|Casting|CastToCombatInterface _returnvalue))
  (bind _output_get (Variables|Default|SetTargetLocation (Transformation|GetActorLocation _returnvalue_4)))
  (Class|CombatInterface|SetFacingTarget _ascombat_interface _output_get)
  (bind _returnvalue_5 (Class|CombatInterface|GetMeleeAttackAnimMontageandTag(Message) (Ability|GetAvatarActorfromActorInfo)))
  (|PlayMontageandWaitProxy "None" (.AttackMontage (Utilities|Struct|BreakMontageTag _returnvalue_5)) 1.0 "None" true 1.0 0.0 false
    (:then
      (Ability|Async|WaitGameplayEventToActor _returnvalue_2 (.MontageTag (Utilities|Struct|BreakMontageTag _returnvalue_5)) true
        (:EventReceived
          (bind _returnvalue_6 (Class|CombatInterface|GetWeaponTipSocketLocation(Message) _returnvalue_2 (.MontageTag (Utilities|Struct|BreakMontageTag _returnvalue_5))))
          (bind _overlapactors (Class|AuraAbilitySystemLibrary|GetLivePlayersWithinRadius _returnvalue_3 (Utilities|Array|MakeArray _returnvalue_3) 5e+01 _returnvalue_6))
          (for _array_element _overlapactors
            (Class|AuraAttackAbility|CauseDamage _array_element)))))
    (:OnCompleted
      (Ability|EndAbility :!label _label))
    (:OnInterrupted
      (goto _label))
    (:OnCancelled
      (goto _label))))

(event Ability|EventOnEndAbility
  (params (bWasCancelled :type Boolean)))