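; GA_RangeAttack is a Gameplay Ability that makes its avatar fire a projectile at its target actor.
; On activation it faces the target's location and plays the attack montage from the avatar's melee montage-and-tag getter.
; The montage tag triggers projectile spawning as a one-shot gameplay event and also selects the socket, aiming at the location captured on activation.
; The ability ends after spawning or when the montage completes, is interrupted or is cancelled.
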(event Ability|EventActivateAbility
  (bind _returnvalue (Ability|GetAvatarActorfromActorInfo))
  (bind _returnvalue_2 (Class|EnemyInterface|GetTargetActor(Message) _returnvalue))
  (bind _ascombat_interface (Utilities|Casting|CastToCombatInterface _returnvalue))
  (bind _output_get (Variables|Default|SetTargetLocation (Transformation|GetActorLocation _returnvalue_2)))
  (Class|CombatInterface|SetFacingTarget _ascombat_interface _output_get)
  (bind _returnvalue_3 (Class|CombatInterface|GetMeleeAttackAnimMontageandTag(Message) (Ability|GetAvatarActorfromActorInfo)))
  (|PlayMontageandWaitProxy "None" (.AttackMontage (Utilities|Struct|BreakMontageTag _returnvalue_3)) 1.0 "None" true 1.0 0.0 false
    (:then
      (Ability|Async|WaitGameplayEventToActor (Ability|GetAvatarActorfromActorInfo) (.MontageTag (Utilities|Struct|BreakMontageTag _returnvalue_3)) true
        (:EventReceived
          (Class|AuraFireSpell|SpawnProjectile (Variables|Default|GetTargetLocation) (.MontageTag (Utilities|Struct|BreakMontageTag _returnvalue_3)))
          (Ability|EndAbility))))
    (:OnCompleted
      (Ability|EndAbility :!label _label))
    (:OnInterrupted
      (goto _label))
    (:OnCancelled
      (goto _label))))

(event Ability|EventOnEndAbility
  (params (bWasCancelled :type Boolean)))