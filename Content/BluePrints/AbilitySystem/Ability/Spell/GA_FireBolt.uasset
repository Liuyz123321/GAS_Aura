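; GA_FireBolt is a gameplay ability that casts a fire bolt spell toward the mouse location.
; On activation it commits, gets target data from a MouseData task, and turns the avatar toward that point through CombatInterface.
; It then plays the FireBolt montage and waits for the Event.Montage.FireBolt gameplay event, which spawns the projectile from a socket tag and ends the ability.
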(event Ability|EventActivateAbility
  (Ability|CommitAbility)
  (bind _mousedata (|MouseData)
    (:ValidData
      (Variables|Default|SetMouseLocation _mousedata)
      (bind _ascombat_interface (Utilities|Casting|CastToCombatInterface (Ability|GetAvatarActorfromActorInfo)))
      (Class|CombatInterface|SetFacingTarget _ascombat_interface (Variables|Default|GetMouseLocation))
      (|PlayMontageandWaitProxy "None" "/Game/Assets/Characters/Aura/Animations/Abilities/Motage_FireBolt.Motage_FireBolt" 1.0 "None" true 1.0 0.0 false
        (:then
          (Ability|Tasks|WaitGameplayEvent "(TagName=\"Event.Montage.FireBolt\")" 0
            (:EventReceived
              (Class|AuraFireSpell|SpawnProjectile (Variables|Default|GetMouseLocation) (Variables|Default|GetSocket%20Tag))
              (Ability|EndAbility))))))))

(event Ability|EventOnEndAbility
  (params (bWasCancelled :type Boolean)))