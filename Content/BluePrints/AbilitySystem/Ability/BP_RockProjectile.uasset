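; BP_RockProjectile is a rock projectile actor in the ability system that tumbles while it exists.
; BeginPlay picks random signed yaw, pitch and roll spin rates, so each instance rotates differently.
; Tick applies those rates as a local rotation scaled by delta time, keeping the spin frame-rate independent.
; The graphs contain only this spin, with no movement, overlap or damage logic.
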(event EventBeginPlay
  (bind _returnvalue (Math|Random|RandomFloatinRange -5e+02 5e+02))
  (Variables|Default|SetYawRot _returnvalue)
  (Variables|Default|SetPitchRot _returnvalue)
  (Variables|Default|SetRollRot _returnvalue))

(event Collision|EventActorBeginOverlap
  (params (OtherActor :type Actor%20Object%20Reference)))

(event EventTick
  (params (DeltaSeconds :type Float%20%28single-precision%29))
  (Transformation|AddActorLocalRotation (Math|Rotator|MakeRotator (* DeltaSeconds (Variables|Default|GetRollRot)) (* DeltaSeconds (Variables|Default|GetPitchRot)) (* DeltaSeconds (Variables|Default|GetYawRot))) false false))

(fn ConstructionScript)