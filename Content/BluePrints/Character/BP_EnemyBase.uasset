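; BP_EnemyBase is the base enemy character Blueprint, handling its health bar display and death-style dissolve effects.
; Mesh and weapon dissolve events wait briefly, then run timelines that drive a Dissolve scalar on the supplied material instance.
; On BeginPlay it binds a progress-bar change delegate that writes the new value into the WBP_EnermyHealthBar widget of its HealthBar component.
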(event Custom|ChangeEnemyProgressBar_事件
  (params (NewData :type Float%20%28single-precision%29))
  (bind _aswbp_enermy_health_bar (Utilities|Casting|CastToWBP_EnermyHealthBar (UserInterface|GetWidget (Variables|Default|GetHealthBar))))
  (Variables|/Game/BluePrints/UI/ProcessBar/EnermyHealthBar/WBP_EnermyHealthBar.WBP_EnermyHealthBar_C|SetEnemyHealthBarProcess _aswbp_enermy_health_bar NewData))

(event EventBeginPlay
  (EventDispatchers|AssignChangeEnemyProgressBar (delegate Custom|ChangeEnemyProgressBar_事件)))

(event Collision|EventActorBeginOverlap
  (params (OtherActor :type Actor%20Object%20Reference)))

(event EventMeshDissolveTimeLine
  (params (MaterialInstance :type Material%20Instance%20Dynamic%20Object%20Reference))
  (Utilities|FlowControl|Delay 2.0)
  (bind _meshdissolve (Timeline|MeshTimeLine Play)
    (:Update
      (Rendering|Material|SetScalarParameterValue MaterialInstance "Dissolve" _meshdissolve :!class /Script/Engine.MaterialInstanceDynamic))))

(event EventWeaponDissolveTimeLine
  (params (MaterialInstance :type Material%20Instance%20Dynamic%20Object%20Reference))
  (Utilities|FlowControl|Delay 2.0)
  (bind _meshdissolve (Timeline|WeaponTimeLine Play)
    (:Update
      (Rendering|Material|SetScalarParameterValue MaterialInstance "Dissolve" _meshdissolve :!class /Script/Engine.MaterialInstanceDynamic))))

(fn ConstructionScript)